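; Sliding door Blueprint that opens and closes as something enters or leaves its Box trigger.
; Box overlap events wait a short Delay before calling open or close, with no check on the overlapping actor.
; The Door timeline plays forward or in reverse, lerping the relative location of Door2 along its local Y axis.
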(event OnComponentEndOverlap(Box)
  (params (OverlappedComponent :type Primitive%20Component%20Object%20Reference) (OtherActor :type Actor%20Object%20Reference) (OtherComp :type Primitive%20Component%20Object%20Reference) (OtherBodyIndex :type Integer))
  (Utilities|FlowControl|Delay 0.2)
  (CallFunction|CloseDoor))

(event OnComponentBeginOverlap(Box)
  (params (OverlappedComponent :type Primitive%20Component%20Object%20Reference) (OtherActor :type Actor%20Object%20Reference) (OtherComp :type Primitive%20Component%20Object%20Reference) (OtherBodyIndex :type Integer) (bFromSweep :type Boolean) (SweepResult :type Hit%20Result%20Structure%20%28by%20ref%29))
  (Utilities|FlowControl|Delay 0.1)
  (CallFunction|OpenDoor))

(event Custom|Open_door
  (bind _door (Timeline|door Play)
    (:Update
      (Transformation|SetRelativeLocation (Variables|Default|Getdoor2) (Math|Vector|Lerp(Vector) "0, 0, 0" "0.000000,300.000000,0.000000" _door) false false))))

(event Custom|Close_door
  (bind _door (Timeline|door Reverse)
    (:Update
      (Transformation|SetRelativeLocation (Variables|Default|Getdoor2) (Math|Vector|Lerp(Vector) "0, 0, 0" "0.000000,300.000000,0.000000" _door) false false))))

(fn ConstructionScript)
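; Player character Blueprint that carries a pistol and can grab, carry, drop and launch physics objects.
; On BeginPlay it spawns BP_WeaponPistol, attaches it to the mesh via the for_pistol socket's bone, and forwards Fire input to it.
; Left mouse grabs a simulating component through a camera line trace or launches the held one by impulse; right mouse drops it.
; A PhysicsHandle follows the Scene component every Tick.
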(event Custom|\drop%20obj
  (Physics|Components|PhysicsHandle|ReleaseComponent (Variables|Default|GetPhysicsHandle))
  (Variables|Default|SetIs%20holding%20obj false))

(event Custom|launch%20obj
  (if (Variables|Default|GetIs%20holding%20obj)
    (CallFunction|\dropObj)
    (Physics|AddImpulse (.HitComponent (Collision|BreakHitResult (stale Custom|pick%20up%20obj _outhit))) (* (Math|Vector|GetForwardVector (Variables|Default|GetFollowCamera)) "24000.000000,24000.000000,24000.000000") "None" false)))

(event Custom|pick%20up%20obj
  (bind _followcamera (Variables|Default|GetFollowCamera))
  (bind _returnvalue (Transformation|GetWorldLocation _followcamera))
  (bind (_outhit _returnvalue_2) (Collision|LineTraceByChannel _returnvalue (+ (* (Math|Vector|GetForwardVector _followcamera) "400000.000000,400000.000000,400000.000000") _returnvalue) "TraceTypeQuery1" false 0 "None"))
  (if _returnvalue_2
    (if (Physics|IsSimulatingPhysics (.HitComponent (Collision|BreakHitResult _outhit)) "None")
      (Physics|Components|PhysicsHandle|GrabComponentatLocationwithRotation (Variables|Default|GetPhysicsHandle) (.HitComponent (Collision|BreakHitResult _outhit)) "None" (Transformation|GetWorldLocation (.HitComponent (Collision|BreakHitResult _outhit))) "0, 0, 0")
      (Variables|Default|SetIs%20holding%20obj true))))

(event Collision|EventActorBeginOverlap
  (params (OtherActor :type Actor%20Object%20Reference)))

(event EventBeginPlay
  (CallFunction|SnapWeapons))

(event EventTick
  (params (DeltaSeconds :type Float%20%28single-precision%29))
  (Physics|Components|PhysicsHandle|SetTargetLocation (Variables|Default|GetPhysicsHandle) (Transformation|GetWorldLocation (Variables|Default|GetScene))))

(event Input|ActionEvents|InputActionFire
  (params (Key :type Key%20Structure :default "None"))
  (bind _current_weapon (Variables|Default|Getcurrent_weapon))
  (:Pressed
    (Default|StartFire _current_weapon))
  (:Released
    (Default|StopFire _current_weapon)))

(event Input|MouseEvents|LeftMouseButton
  (params (Key :type Key%20Structure :default "None"))
  (:Pressed
    (if (Variables|Default|GetIs%20holding%20obj)
      (CallFunction|LaunchObj)
      (else
        (CallFunction|PickUpObj)))))

(event Input|MouseEvents|RightMouseButton
  (params (Key :type Key%20Structure :default "None"))
  (:Pressed
    (if (Variables|Default|GetIs%20holding%20obj)
      (CallFunction|\dropObj))))

(fn ConstructionScript)

(fn SnapWeapons
  (bind _mesh (Variables|Character|GetMesh))
  (bind _returnvalue (Game|SpawnActorfromClass "/Game/Weapon/BP_Weapon-Pistol.BP_Weapon-Pistol_C" (Transformation|GetSocketTransform _mesh "for_pistol" "RTS_ParentBoneSpace") "Undefined" 0 0))
  (bind _output_get (Variables|Default|Setcurrent_weapon _returnvalue))
  (Transformation|AttachComponentToComponent _output_get (Variables|Character|GetMesh) (Class|SkinnedMeshComponent|GetSocketBoneName _mesh "for_pistol") "KeepRelative" "KeepRelative" "KeepRelative" true)
  (Variables|/Game/Weapon/BP_Weapon-Base.BP_Weapon-Base_C|SetCharRef _output_get self))
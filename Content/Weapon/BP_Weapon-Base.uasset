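; Base weapon Blueprint that loads its stats from DT_Weapon at construction and fires BP_Bullet projectiles.
; StartFire handles only Single mode, opening a gate that re-enters after each FireRate delay until StopFire toggles it.
; Aim comes from a follow-camera trace against WorldStatic, turned into a muzzle-to-target rotation.
; Random spread offsets that rotation only in the negative direction before each bullet spawns.
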(event Custom|StartFire
  (switch Utilities|FlowControl|Switch|SwitchonEnum_FireMode (Variables|Default|GetFireMode)
    (:NewEnumerator0
      (Utilities|FlowControl|Sequence
        (:then_0
          (goto _label Open))
        (:then_1
          (Utilities|FlowControl|Gate true :!label _label
            (:Exit
              (Utilities|FlowControl|Sequence
                (:then_0
                  (Utilities|FlowControl|RetriggerableDelay (Variables|Default|GetFire%20Rate))
                  (goto _label))
                (:then_1
                  (CallFunction|SpawnProjectile))))))))))

(event Custom|StopFire
  (Utilities|FlowControl|Gate true) ; enters at Toggle
)

(event Collision|EventActorBeginOverlap
  (params (OtherActor :type Actor%20Object%20Reference)))

(event EventTick
  (params (DeltaSeconds :type Float%20%28single-precision%29)))

(fn ConstructionScript
  (bind _returnvalue (Utilities|GetDataTableRow "/Game/Weapon/DT_Weapon.DT_Weapon" (Variables|Default|GetWeaponRownName))
    (:then
      (bind _output_get (Variables|Default|SetWeaponData _returnvalue))
      (Variables|Default|SetFireMode (.FireMode (Utilities|Struct|BreakStruct_WeaponData _output_get)))
      (Variables|Default|SetMuzzle%20Name (.MuzzleName (Utilities|Struct|BreakStruct_WeaponData _output_get)))
      (Variables|Default|SetFire%20Rate (.FireRate (Utilities|Struct|BreakStruct_WeaponData _output_get)))
      (Variables|Default|SetReload%20Delay (.ReloadDelay (Utilities|Struct|BreakStruct_WeaponData _output_get)))
      (Variables|Default|SetWeapon%20Spread (.WeaponSpread (Utilities|Struct|BreakStruct_WeaponData _output_get))))))

(fn CalculateDirection
  (bind _returnvalue (Utilities|MuzzlePosition))
  (bind _weaponcamera (Variables|Default|GetWeaponCamera))
  (bind _charref (Variables|Default|GetCharRef))
  (bind _followcamera (Variables|/Script/Orion.CharacterCPP|GetFollowCamera _charref))
  (bind _returnvalue_2 (select false _weaponcamera _followcamera))
  (bind _returnvalue_3 (Transformation|GetWorldRotation _returnvalue_2))
  (bind _returnvalue_4 (Transformation|GetWorldLocation _returnvalue_2))
  (bind _end (|EndPoint _returnvalue_4 _returnvalue_3))
  (bind (_outhit _returnvalue_5) (Collision|LineTraceForObjects (|StartPoint _returnvalue_3 _returnvalue_4) _end (Utilities|Array|MakeArray "ObjectTypeQuery1") true 0 "ForDuration"))
  (return _returnvalue (Math|Rotator|FindLookatRotation _returnvalue (Math|Vector|SelectVector (.ImpactPoint (Collision|BreakHitResult _outhit)) _end _returnvalue_5))))

(fn SpawnProjectile
  (bind (_location _rotation) (CallFunction|CalculateDirection))
  (bind _transform (CallFunction|CalculateFinalDirection _location _rotation))
  (Game|SpawnActorfromClass "/Game/Weapon/BP_Bullet.BP_Bullet_C" _transform "Undefined" 0 0))

(fn CalculateFinalDirection
  (params (Location :type Vector) (Rotation :type Rotator))
  (bind _weapon_spread (Variables|Default|GetWeapon%20Spread))
  (bind _returnvalue (* _weapon_spread -1.0))
  (return (Math|Transform|MakeTransform Location (Math|Rotator|CombineRotators Rotation (Math|Rotator|MakeRotator (Math|Random|RandomFloatinRange _returnvalue 0.0) (Math|Random|RandomFloatinRange _returnvalue 0.0) (Math|Random|RandomFloatinRange _returnvalue 0.0))))))